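; BP_OrangeSpawner is an actor that spawns BP_Orange actors at its own transform, up to a capped count.
; Each call to the 오렌지스폰 event increments the 오렌지 counter and spawns one orange, doing nothing once the counter reaches the limit of about twenty.
; The construction script sets the text on 오렌지스폰 to the actor's display name.
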(event `오렌지스폰`
  (if (not (>= (`self.오렌지`) 19.5))
    (set `self.오렌지` (+ (`self.오렌지`) 1.0))
    (`|SpawnActorFromClass` "/Game/Test/TEST0822/BP_Orange.BP_Orange_C" (`self.GetTransform`) "Undefined" "MultiplyWithRoot" null null)))

(fn `UserConstructionScript`
  (`TextRenderComponent.K2_SetText` (`self. 오렌지스폰`) (`KismetTextLibrary.Conv_StringToText` (`KismetSystemLibrary.GetDisplayName` self))))