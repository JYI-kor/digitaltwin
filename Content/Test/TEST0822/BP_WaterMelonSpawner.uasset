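; BP_WaterMelonSpawner is a test spawner actor that creates watermelons up to a limit.
; Each DoSpawn call increments a float counter (수박갯수, watermelon count) and spawns one SpawnActorClass actor at the spawner's transform, until the counter reaches 9.5.
; The counter is never decremented here, so the limit applies to total spawns rather than live watermelons.
; The construction script labels the spawner by writing its display name into a TextRender component.
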(event `DoSpawn`
  ; 수박의 갯수가 9.5개 이상인가?
  (if (not (>= (`self.수박갯수`) 9.5))
    ; 수박을 1개씩 스폰한다.
    (set `self.수박갯수` (+ (`self.수박갯수`) 1.0))
    (`|SpawnActorFromClass` (`self.SpawnActorClass`) (`self.GetTransform`) "Undefined" "MultiplyWithRoot" null null)))

(fn `UserConstructionScript`
  (`TextRenderComponent.K2_SetText` (`self.TextRender`) (`KismetTextLibrary.Conv_StringToText` (`KismetSystemLibrary.GetDisplayName` self))))