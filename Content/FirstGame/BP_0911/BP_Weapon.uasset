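; BP_Weapon is a weapon actor that sits in the world as a physics object and can be attached to or detached from a character.
; Its mesh and data come from DT_Weapon, using RowName in the construction script or a random row at BeginPlay when RowName is None.
; AttachToCharacter disables physics and snaps to the row's socket on the character mesh, while DetachToCharacter detaches and re-enables physics.
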(event `self.ReceiveBeginPlay`
  (`PrimitiveComponent.SetSimulatePhysics` (`self.Weapon`) true)
  (if (== (`self.Row Name`) "None")
    (`self.Random Weapon`)))

(fn `Attach To Character`
  (params (Character :type "Character Object Reference"))
  (bind (_weapon_data_staticmesh _weapon_data_name _weapon_data_damage _weapon_data_socketname) (break `/Game/FirstGame/BP_0911/ST_Weapon` (`self.Weapon Data`)))
  (`PrimitiveComponent.SetSimulatePhysics` (`self.Weapon`) false)
  (`self.K2_AttachToComponent` (`Character.Mesh` Character) _weapon_data_socketname "SnapToTarget" "SnapToTarget" "KeepWorld"))

(fn `Detach To Character`
  (`self.K2_DetachFromActor` "KeepWorld" "KeepWorld" "KeepWorld")
  (`PrimitiveComponent.SetSimulatePhysics` (`self.Weapon`) true))

(fn `Random Weapon`
  (bind _outrownames (`DataTableFunctionLibrary.GetDataTableRowNames` "/Game/FirstGame/BP_0911/DT_Weapon.DT_Weapon"))
  (bind _returnvalue (`|GetDataTableRow` "/Game/FirstGame/BP_0911/DT_Weapon.DT_Weapon" (`KismetArrayLibrary.Array_Random` _outrownames))
    (:`then`
      (bind _output_get (set `self.Weapon Data` _returnvalue))
      (`StaticMeshComponent.SetStaticMesh` (`self.Weapon`) (`.StaticMesh_6_0974708942D96281DAB5138A3E038069` (break `/Game/FirstGame/BP_0911/ST_Weapon` _output_get))))))

(fn `UserConstructionScript`
  (bind _returnvalue (`|GetDataTableRow` "/Game/FirstGame/BP_0911/DT_Weapon.DT_Weapon" (`self.Row Name`))
    (:`then`
      (bind _output_get (set `self.Weapon Data` _returnvalue))
      (`StaticMeshComponent.SetStaticMesh` (`self.Weapon`) (`.StaticMesh_6_0974708942D96281DAB5138A3E038069` (break `/Game/FirstGame/BP_0911/ST_Weapon` _output_get))))))