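; BP_Dummy is a damageable target dummy with a health widget that respawns after being depleted.
; AnyDamage lowers HP, clamps it at zero and sends non-negative results to the DummyWidget.
; At zero it hides the cube and widget, disables collision, and a five-second timer calls Show Dummy to restore them at full health.
; Tick rotates the widget to face the player camera.
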(event `self.ReceiveBeginPlay`
  (`self.Begin Show HP`))

(event `self.ReceiveAnyDamage`
  (params (Damage :type "Float (single-precision)") (DamageType :type "DamageType Object Reference") (InstigatedBy :type "Controller Object Reference") (DamageCauser :type "Actor Object Reference"))
  (`self.Add Damage` Damage)
  (if (== (`self.HP`) 0.0)
    (`self.Hide Dummy`)
    (`KismetSystemLibrary.K2_SetTimer` null "Show Dummy" 5.0)))

(event `self.ReceiveTick`
  (params (DeltaSeconds :type "Float (single-precision)"))
  (`SceneComponent.K2_SetWorldRotation` (`self.Widget`) (`KismetMathLibrary.FindLookAtRotation` (`SceneComponent.K2_GetComponentLocation` (`self.Widget`)) (`self.K2_GetActorLocation` (`GameplayStatics.GetPlayerCameraManager` 0))) false false))

(fn `Add Damage`
  (params (Damage :type "Float (double-precision)"))
  (bind _output_get (set `self.HP` (- (`self.HP`) Damage)))
  (if (< (`self.HP`) 0.0)
    (set `self.HP` 0.0)
    (else
      (bind _asdummy_widget (cast `/Game/FirstGame/BP_0911/DummyWidget` (`WidgetComponent.GetUserWidgetObject` (`self.Widget`))))
      (`/Game/FirstGame/BP_0911/DummyWidget.Update HP` _asdummy_widget (`KismetMathLibrary.FFloor` _output_get)))))

(fn `Begin Show HP`
  (bind _asdummy_widget (cast `/Game/FirstGame/BP_0911/DummyWidget` (`WidgetComponent.GetUserWidgetObject` (`self.Widget`))))
  (`/Game/FirstGame/BP_0911/DummyWidget.Update HP` _asdummy_widget (`KismetMathLibrary.FTrunc` (`self.HP`))))

(fn `Hide Dummy`
  (`SceneComponent.SetVisibility` (`self.Cube`) false false)
  (`PrimitiveComponent.SetCollisionEnabled` (`self.Cube`) "NoCollision")
  (`SceneComponent.SetVisibility` (`self.Widget`) false false))

(fn `Set HP 100`
  (bind _asdummy_widget (cast `/Game/FirstGame/BP_0911/DummyWidget` (`WidgetComponent.GetUserWidgetObject` (`self.Widget`))))
  (`/Game/FirstGame/BP_0911/DummyWidget.Max HP` _asdummy_widget)
  (set `self.HP` 100.0))

(fn `Show Dummy`
  (`SceneComponent.SetVisibility` (`self.Cube`) true false)
  (`PrimitiveComponent.SetCollisionEnabled` (`self.Cube`) "QueryAndPhysics")
  (`SceneComponent.SetVisibility` (`self.Widget`) true false)
  (`self.Set HP 100`))

(fn `UserConstructionScript`)