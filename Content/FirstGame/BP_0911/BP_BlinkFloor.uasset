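; BP_BlinkFloor is a floor actor that temporarily disappears after something hits it.
; A component hit on the Floor starts a short timer that calls Hide Floor, which turns off its visibility and collision.
; Hide Floor then schedules Show Floor by function-name timer, restoring visibility and query-and-physics collision after a longer delay.
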(event `self.Floor.OnComponentHit`
  (params (HitComponent :type "PrimitiveComponent Object Reference") (OtherActor :type "Actor Object Reference") (OtherComp :type "PrimitiveComponent Object Reference") (NormalImpulse :type "Vector Structure") (Hit :type "HitResult Structure (by ref)"))
  (`KismetSystemLibrary.K2_SetTimer` null "Hide Floor" 2.0))

(fn `Hide Floor`
  (`SceneComponent.SetVisibility` (`self.Floor`) false false)
  (`PrimitiveComponent.SetCollisionEnabled` (`self.Floor`) "NoCollision")
  (`KismetSystemLibrary.K2_SetTimer` null "Show Floor" 5.0))

(fn `Show Floor`
  (`SceneComponent.SetVisibility` (`self.Floor`) true false)
  (`PrimitiveComponent.SetCollisionEnabled` (`self.Floor`) "QueryAndPhysics"))

(fn `UserConstructionScript`)