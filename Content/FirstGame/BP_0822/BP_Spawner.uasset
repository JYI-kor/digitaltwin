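; BP_Spawner is an actor that spawns a BP_Chair at its own transform when a linked switch turns on.
; On BeginPlay it binds a handler to the Switch reference's update event dispatcher, and that handler calls the DoSpawn event only for the on state.
; The construction script sets a TextRender to the spawner's display name as a label.
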(event `self.ReceiveBeginPlay`
  (add `/Game/FirstGame/BP_0909/BP_SwitchBase.NewEventDispatcher_Update Switch` (`self.Switch`) (`|CreateDelegate` :!event `Event Update Swtich`)))

(event `DoSpawn`
  (`|SpawnActorFromClass` "/Game/FirstGame/BP_0822/BP_Chair.BP_Chair_C" (`self.GetTransform`) "Undefined" "MultiplyWithRoot" null null))

(fn `Event Update Swtich`
  (params (`Is Switch On` :type Boolean))
  (if `Is Switch On`
    (`self.DoSpawn`)))

(fn `UserConstructionScript`
  (`TextRenderComponent.K2_SetText` (`self.TextRender`) (`KismetTextLibrary.Conv_StringToText` (`KismetSystemLibrary.GetDisplayName` self))))