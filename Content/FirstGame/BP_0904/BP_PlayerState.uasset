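; Player state Blueprint that tracks a player's health (HP) and shield (SH) and broadcasts each change through event dispatchers.
; Damage drains the shield first and passes the overflow to HP, and is ignored once HP reaches zero.
; Healing restores HP, or the shield when HP is full, clamping to a hard-coded 100 rather than the max variables.
; BeginPlay calls the revive function, which refills both pools.
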(event `self.ReceiveBeginPlay`
  (`self.Do Revive PlayerState`))

(fn `Add Damage(HP)`
  (params (Damage :type "Float (double-precision)"))
  (if (not (`self.IsDeath`))
    (bind _reamin_damage (`self.Add Damage(SH)` Damage))
    (set `self.Current HP` (`KismetMathLibrary.FClamp` (- (`self.Current HP`) _reamin_damage) 0.0 100.0))
    (`self.NewEventDispatcher_Update HP` (`self.Current HP`) (`self.Max HP`))))

(fn `Add Damage(SH)`
  (params (Damage :type "Float (double-precision)"))
  (returns (`Reamin Damage` :type "Float (double-precision)"))
  (locals (`Temp SH` :type "Float (double-precision)"))
  (if (not (`self.IsDeath`))
    (bind _output_get (set `local.Temp SH` (- (`self.Current SH`) Damage)))
    (set `self.Current SH` (`KismetMathLibrary.FClamp` _output_get 0.0 100.0))
    (`self.NewEventDispatcher_Update SH` (`self.Current SH`) (`self.Max SH`))
    (if (< (`local.Temp SH`) 0.0)
      (return (`KismetMathLibrary.Abs` (`local.Temp SH`)))
      (else
        (return 0.0)))))

(fn `Do Revive PlayerState`
  (`|ExecutionSequence`
    (:`then_0`
      (set `self.Current SH` (`self.Max SH`))
      (`self.NewEventDispatcher_Update SH` (`self.Current SH`) (`self.Max SH`)))
    (:`then_1`
      (set `self.Current HP` (`self.Max HP`))
      (`self.NewEventDispatcher_Update HP` (`self.Current HP`) (`self.Max HP`)))))

(fn `Heal HP`
  (params (Heal :type "Float (double-precision)"))
  (if (>= (`self.Current HP`) 100.0)
    (if (<= (`self.Current SH`) 100.0)
      (set `self.Current SH` (`KismetMathLibrary.FClamp` (+ (`self.Current SH`) Heal) 0.0 100.0))
      (`self.NewEventDispatcher_Update SH` (`self.Current SH`) (`self.Max SH`)))
    (elif (not (`self.IsDeath`))
      (set `self.Current HP` (`KismetMathLibrary.FClamp` (+ (`self.Current HP`) Heal) 0.0 100.0))
      (`self.NewEventDispatcher_Update HP` (`self.Current HP`) (`self.Max HP`)))))

(fn `IsDeath`
  (returns (`Is Death` :type Boolean))
  (return (<= (`self.Current HP`) 0.0)))

(fn `UserConstructionScript`)