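; BP_Canon is a cannon actor that automatically fires Bullet actors at a fixed interval.
; A looping function-name timer calls Do Shoot, which spawns a Bullet at the Arrow component's world location and rotation.
; Toggle Shoot starts or clears that timer from the Toggle flag, applied on BeginPlay and flipped whenever F is pressed.
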(event `self.ReceiveBeginPlay`
  (`self.Toggle Shoot` (`self.Toggle`)))

(event `/Game/FirstGame/BP_0828/BPI_Switch.Press F`
  (bind _output_get (set `self.Toggle` (not (`self.Toggle`))))
  (`self.Toggle Shoot` _output_get))

(fn `Do Shoot`
  (bind _arrow (`self.Arrow`))
  (`|SpawnActorFromClass` (`self.Bullet`) (`KismetMathLibrary.MakeTransform` (`SceneComponent.K2_GetComponentLocation` _arrow) (`SceneComponent.K2_GetComponentRotation` _arrow)) "Undefined" "MultiplyWithRoot" null null))

(fn `Toggle Shoot`
  (params (Toggle :type Boolean))
  (if Toggle
    (`KismetSystemLibrary.K2_SetTimer` null "Do Shoot" 1.0 true)
    (else
      (`KismetSystemLibrary.K2_ClearTimer` null "Do Shoot"))))

(fn `UserConstructionScript`)