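; BP_Counter1 is a counter Blueprint that shows a number on a widget component in the world.
; Tick rotates the widget to face the player camera.
; PressF flips a toggle and, on every other press, increments Count, wrapping to zero above nine, then passes it to the CountWidget.
; PlayAndStop is an empty stub, and older decrement and text-setting logic is left unconnected.
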(event `self.ReceiveTick`
  (params (DeltaSeconds :type "Float (single-precision)"))
  (`SceneComponent.K2_SetWorldRotation` (`self.Widget`) (`KismetMathLibrary.FindLookAtRotation` (`SceneComponent.K2_GetComponentLocation` (`self.Widget`)) (`self.K2_GetActorLocation` (`GameplayStatics.GetPlayerCameraManager` 0))) false false))

(event `/Game/FirstGame/BP_0828/BPI_Switch.Press F`
  (bind _output_get (set `self.Toggle` (not (`self.Toggle`))))
  (if _output_get
    (`self.Update Count`)
    (bind _ascount_widget (cast `/Game/FirstGame/BP_0910/CountWidget` (`WidgetComponent.GetUserWidgetObject` (`self.Widget`))))
    (`/Game/FirstGame/BP_0910/CountWidget.Update Count` _ascount_widget (`self.Count`))))

(fn `Play and Stop`
  (params (`Is Play` :type Boolean))
  (returns (bResult :type Boolean)))

(fn `Update Count`
  ; Count를 1증가
  (set `self.Count` (+ (`self.Count`) 1))
  ; Count가 9보다 크면 0으로 초기화
  (if (> (`self.Count`) 9)
    (set `self.Count` 0)))

(fn `UserConstructionScript`)