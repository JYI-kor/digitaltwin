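; Cannonball projectile that launches itself forward with a physics impulse on spawn and expires after a short delay.
; On hit, DoExplosion spawns particles and sound, applies radial damage, draws a debug sphere and destroys the actor.
; DoImpluseTarget then knocks a hit Character back using the inverted, scaled hit impulse.
; A hit BP_MilitaryA07Character is also switched to ragdoll.
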(event `self.ReceiveBeginPlay`
  (bind _canonball (`self.CanonBall`))
  (`PrimitiveComponent.AddImpulse` _canonball (* (`SceneComponent.GetForwardVector` _canonball) 300000.0) "None" false)
  (`KismetSystemLibrary.Delay` 5.0)
  (`self.K2_DestroyActor`))

(event `self.CanonBall.OnComponentHit`
  (params (HitComponent :type "PrimitiveComponent Object Reference") (OtherActor :type "Actor Object Reference") (OtherComp :type "PrimitiveComponent Object Reference") (NormalImpulse :type "Vector Structure") (Hit :type "HitResult Structure (by ref)"))
  (`|ExecutionSequence`
    (:`then_0`
      (`self.Do Explosion` OtherActor)
      (`self.Do Impluse Target` OtherActor NormalImpulse)
      (bind _asbp_military_a07character (cast `/Game/ThirdPerson/Blueprints/BP_MilitaryA07Character` OtherActor))
      (`/Game/ThirdPerson/Blueprints/BP_MilitaryA07Character.Do Ragdoll` _asbp_military_a07character true))))

(fn `Do Explosion`
  (params (`Other Actor` :type "Actor Object Reference"))
  (bind _returnvalue_location (`KismetMathLibrary.BreakTransform` (`SceneComponent.K2_GetComponentToWorld` (`self.CanonBall`))))
  (bind (_returnvalue_location_2 _returnvalue_rotation) (`KismetMathLibrary.BreakTransform` (`SceneComponent.K2_GetComponentToWorld` (`self.CanonBall`))))
  (`GameplayStatics.SpawnEmitterAtLocation` "/Game/StarterContent/Particles/P_Explosion.P_Explosion" _returnvalue_location_2 _returnvalue_rotation (5.0 5.0 5.0))
  (`GameplayStatics.ApplyRadialDamage` 20.0 (`SceneComponent.K2_GetComponentLocation` (`self.CanonBall`)) 500.0 null (`|MakeArray` self :!type "Actor Object Reference") self null)
  (`GameplayStatics.SpawnSoundAtLocation` "/Game/StarterContent/Audio/Explosion_Cue.Explosion_Cue" _returnvalue_location (struct) 1.0 1.0 0.0 null null)
  (`KismetSystemLibrary.DrawDebugSphere` (`SceneComponent.K2_GetComponentLocation` (`self.CanonBall`)) 500.0 12 (struct :`R` 1.0 :`A` 1.0) 1.0 1.0)
  (`self.K2_DestroyActor`))

(fn `Do Impluse Target`
  (params (OtherActor :type "Object Object Reference") (`Normal Impluse` :type "Vector Structure"))
  (bind _ascharacter (cast `Character` OtherActor))
  (`CharacterMovementComponent.AddImpulse` (`Character.CharacterMovement` _ascharacter) (* `Normal Impluse` -2.0) false))

(fn `UserConstructionScript`)