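; BP_Switch235 is a toggle switch actor with an on/off state and a world-space widget.
; PressF flips IsSwitchOn and calls SwitchOn or SwitchOff to match the new state.
; Every tick, the widget rotates to face the player camera, billboard-style, using a look-at rotation toward the camera manager's location.
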(event `/Game/FirstGame/BP_0828/BPI_Switch.Press F`
  (bind _output_get (set `self.Is Switch On` (not (`self.Is Switch On`))))
  (if _output_get
    (`self.Switch On`)
    (else
      (`self.Switch Off`))))

(event `self.ReceiveTick`
  (params (DeltaSeconds :type "Float (single-precision)"))
  (`SceneComponent.K2_SetWorldRotation` (`self.Widget`) (`KismetMathLibrary.FindLookAtRotation` (`SceneComponent.K2_GetComponentLocation` (`self.Widget`)) (`self.K2_GetActorLocation` (`GameplayStatics.GetPlayerCameraManager` 0))) false false))

(fn `UserConstructionScript`)