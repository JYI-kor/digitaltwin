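; BP_SwitchPhysics is a switch that turns on and off as its SwitchBtn component enters and leaves the Box trigger.
; The overlap events call SwitchOn and SwitchOff, which are not defined in this Blueprint.
; DoPlay and DoStop hold disconnected loops that would send BPI_PlayStop messages to array elements, so they currently do nothing.
; Its own PlayAndStop is a stub returning false.
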(event `self.Box.OnComponentBeginOverlap`
  (params (OverlappedComponent :type "PrimitiveComponent Object Reference") (OtherActor :type "Actor Object Reference") (OtherComp :type "PrimitiveComponent Object Reference") (OtherBodyIndex :type Integer) (bFromSweep :type Boolean) (SweepResult :type "HitResult Structure (by ref)"))
  (if (== OtherComp (`self.SwitchBtn`))
    (`self.Switch On`)))

(event `self.Box.OnComponentEndOverlap`
  (params (OverlappedComponent :type "PrimitiveComponent Object Reference") (OtherActor :type "Actor Object Reference") (OtherComp :type "PrimitiveComponent Object Reference") (OtherBodyIndex :type Integer))
  (if (== OtherComp (`self.SwitchBtn`))
    (`self.Switch Off`)))

(fn `Do Play`
  (params (A :type "Object Object Reference"))
  (if (== A (`self.SwitchBtn`))
    _))

(fn `Do Stop`
  (params (A :type "Object Object Reference"))
  (if (== A (`self.SwitchBtn`))
    _))

(fn `Play and Stop`
  (params (`Is Play` :type Boolean))
  (returns (bResult :type Boolean))
  (return false))

(fn `UserConstructionScript`)