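; Blueprint that slides its Cube back and forth along relative X while a linked switch is on.
; On BeginPlay it binds to the switch's update dispatcher, whose handler starts or stops the movement.
; A Timeline scales the X offset, and each finish flips the Isright flag and loops back to choose Play or Reverse, giving continuous ping-pong motion.
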(event `self.ReceiveBeginPlay`
  (add `/Game/FirstGame/BP_0909/BP_SwitchBase.NewEventDispatcher_Update Switch` (`self.Swtich`) (`|CreateDelegate` :!event `Event Update Swtich`)))

(event `DoPlay`
  (if (`self.Isright`) :!label _label
    (bind (_direction _value) (`Timeline|타임라인` :!label _label_2)
      (:`Update`
        (`SceneComponent.K2_SetRelativeLocation` (`self.Cube`) (* _value (500.0 0.0 0.0)) false false))
      (:`Finished`
        ; not 부울은 앞의 get의 인자를 반대로 인식하게 준다.
        (set `self.Isright` (not (`self.Isright`)))
        (goto _label)))
    (else
      (goto _label_2 :!via `Reverse`))))

(event `DoStop`
  (goto _label_2 :!via `Stop`))

(fn `Event Update Swtich`
  (params (`Is Switch On` :type Boolean))
  (if `Is Switch On`
    (`self.DoPlay`)
    (else
      (`self.DoStop`))))

(fn `UserConstructionScript`)