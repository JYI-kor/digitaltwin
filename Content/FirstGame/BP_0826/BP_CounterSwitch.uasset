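; BP_CounterSwitch is a trigger switch that counts overlaps on Cube1 and toggles the actors in its Actors array.
; Each overlap increments Count, wrapping to zero after nine, and updates the TextRender display.
; Odd counts start BPI_PlayStop actors, or trigger spawning on other actors via BPI_Spawn; even counts stop BPI_PlayStop actors.
; Interface casts keep the switch independent of target classes.
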(event `self.ReceiveBeginPlay`
  (`self.Show Count`))

(event `self.cube1.OnComponentBeginOverlap`
  (params (OverlappedComponent :type "PrimitiveComponent Object Reference") (OtherActor :type "Actor Object Reference") (OtherComp :type "PrimitiveComponent Object Reference") (OtherBodyIndex :type Integer) (bFromSweep :type Boolean) (SweepResult :type "HitResult Structure (by ref)"))
  (`|ExecutionSequence`
    (:`then_0`
      (`self.Show Count Up`))
    (:`then_1`
      (if (== (mod (`self.Count`) 2) 1)
        (`self.Do play and Spawn`)
        (else
          (`self.Do Stop`))))))

(fn `Count 1 Up`
  ; Count를 1증가
  (set `self.Count` (+ (`self.Count`) 1)))

(fn `Do play and Spawn`
  ; Count가 홀수일경우
  (for _array_element (`self.Actors`)
    (bind _asbpi_play_stop (cast `/Game/FirstGame/BP_0827/BPI_PlayStop` _array_element)
      (:`then`
        (`/Game/FirstGame/BP_0827/BPI_PlayStop.Play and Stop` _asbpi_play_stop true))
      (:`CastFailed`
        (bind _asbpi_spawn (cast `/Game/FirstGame/BP_0827/BPI_Spawn` _array_element))
        (`/Game/FirstGame/BP_0827/BPI_Spawn.DoSpawn` _asbpi_spawn)))))

(fn `Do Stop`
  ; Count가 짝수일경우
  (for _array_element (`self.Actors`)
    (bind _asbpi_play_stop (cast `/Game/FirstGame/BP_0827/BPI_PlayStop` _array_element))
    (`/Game/FirstGame/BP_0827/BPI_PlayStop.Play and Stop` _asbpi_play_stop false)))

(fn `Over 9 Count 0`
  ; Count가 9보다 크면
  (if (> (`self.Count`) 9)
    ; Count 0으로 변경
    (set `self.Count` 0)))

(fn `Play and Stop`
  (params (`Is Play` :type Boolean))
  (returns (bResult :type Boolean))
  (return false))

(fn `Show Count`
  ; Count값을 Text Render에 표시
  (`TextRenderComponent.K2_SetText` (`self.TextRender`) (`KismetTextLibrary.Conv_IntToText` (`self.Count`) false true 1 244)))

(fn `Show Count begin`
  ; 시작할 때 Count값을 Text Render에 표시.
  (`TextRenderComponent.K2_SetText` (`self.TextRender`) (`KismetTextLibrary.Conv_IntToText` (`self.Count`) false true 1 244)))

(fn `Show Count Up`
  ; Count증가 표시
  (`self.Count 1 Up`)
  (`self.Over 9 Count 0`)
  (`self.Show Count`))

(fn `UserConstructionScript`)