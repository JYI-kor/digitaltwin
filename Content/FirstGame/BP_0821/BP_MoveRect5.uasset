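; BP_MoveRect5 moves its Sphere component along a two-step staircase in the XZ plane, then back along the same steps, in an endless loop.
; Tick switches on the MoveR state to call one of eight move functions, one per segment.
; Each function nudges the relative location by a fixed amount per frame, so speed depends on frame rate, and sets the next state upon passing its axis threshold.
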(event `self.ReceiveTick`
  (params (DeltaSeconds :type "Float (single-precision)"))
  (switch `/Game/FirstGame/BP_0821/ENUM_MoveType5` (`self.MoveR`)
    (:`NewEnumerator0`
      (`self.MoveUp`))
    (:`NewEnumerator1`
      (`self.MoveRight`))
    (:`NewEnumerator2`
      (`self.MoveUp2`))
    (:`NewEnumerator3`
      (`self.Move Right2`))
    (:`NewEnumerator4`
      (`self.Move Left`))
    (:`NewEnumerator5`
      (`self.Move Down`))
    (:`NewEnumerator6`
      (`self.Move Left2`))
    (:`NewEnumerator7`
      (`self.Move Down2`))))

(fn `Move Down`
  (bind (_relativelocation_x _relativelocation_y _relativelocation_z) (`KismetMathLibrary.BreakVector` (`SceneComponent.RelativeLocation` (`self.Sphere`))))
  ; 아래쪽으로 이동한다.
  (set `self.MoveR` "NewEnumerator5")
  (`SceneComponent.K2_AddRelativeLocation` (`self.Sphere`) (0.0 0.0 -5.0) false false)
  (if (<= _relativelocation_z 100.0)
    (set `self.MoveR` "NewEnumerator6")))

(fn `Move Down2`
  (bind (_relativelocation_x _relativelocation_y _relativelocation_z) (`KismetMathLibrary.BreakVector` (`SceneComponent.RelativeLocation` (`self.Sphere`))))
  ; 아래쪽으로 이동한다.
  (set `self.MoveR` "NewEnumerator7")
  (`SceneComponent.K2_AddRelativeLocation` (`self.Sphere`) (0.0 0.0 -5.0) false false)
  (if (<= _relativelocation_z 0.0)
    (set `self.MoveR` "NewEnumerator0")))

(fn `Move Left`
  (bind _relativelocation_x (`KismetMathLibrary.BreakVector` (`SceneComponent.RelativeLocation` (`self.Sphere`))))
  ; 왼쪽으로 이동한다
  (set `self.MoveR` "NewEnumerator4")
  (`SceneComponent.K2_AddRelativeLocation` (`self.Sphere`) (-5.0 0.0 0.0) false false)
  (if (<= _relativelocation_x 100.0)
    (set `self.MoveR` "NewEnumerator5")))

(fn `Move Left2`
  (bind _relativelocation_x (`KismetMathLibrary.BreakVector` (`SceneComponent.RelativeLocation` (`self.Sphere`))))
  ; 왼쪽으로 이동한다.
  (set `self.MoveR` "NewEnumerator6")
  (`SceneComponent.K2_AddRelativeLocation` (`self.Sphere`) (-5.0 0.0 0.0) false false)
  (if (<= _relativelocation_x 0.0)
    (set `self.MoveR` "NewEnumerator7")))

(fn `Move Right2`
  (bind _relativelocation_x (`KismetMathLibrary.BreakVector` (`SceneComponent.RelativeLocation` (`self.Sphere`))))
  ; 오른쪽으로 이동한다.
  (set `self.MoveR` "NewEnumerator3")
  (`SceneComponent.K2_AddRelativeLocation` (`self.Sphere`) (5.0 0.0 0.0) false false)
  (if (>= _relativelocation_x 200.0)
    (set `self.MoveR` "NewEnumerator4")))

(fn `MoveRight`
  (bind _relativelocation_x (`KismetMathLibrary.BreakVector` (`SceneComponent.RelativeLocation` (`self.Sphere`))))
  ; 오른쪽으로 이동한다.
  (set `self.MoveR` "NewEnumerator1")
  (`SceneComponent.K2_AddRelativeLocation` (`self.Sphere`) (5.0 0.0 0.0) false false)
  (if (>= _relativelocation_x 100.0)
    (set `self.MoveR` "NewEnumerator2")))

(fn `MoveUp`
  (bind (_relativelocation_x _relativelocation_y _relativelocation_z) (`KismetMathLibrary.BreakVector` (`SceneComponent.RelativeLocation` (`self.Sphere`))))
  ; 위쪽으로 이동한다.
  (set `self.MoveR` "NewEnumerator0")
  (`SceneComponent.K2_AddRelativeLocation` (`self.Sphere`) (0.0 0.0 5.0) false false)
  (if (>= _relativelocation_z 100.0)
    (set `self.MoveR` "NewEnumerator1")))

(fn `MoveUp2`
  (bind (_relativelocation_x _relativelocation_y _relativelocation_z) (`KismetMathLibrary.BreakVector` (`SceneComponent.RelativeLocation` (`self.Sphere`))))
  ; 위쪽으로 이동한다.
  (set `self.MoveR` "NewEnumerator2")
  (`SceneComponent.K2_AddRelativeLocation` (`self.Sphere`) (0.0 0.0 5.0) false false)
  (if (>= _relativelocation_z 200.0)
    (set `self.MoveR` "NewEnumerator3")))

(fn `UserConstructionScript`)