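; BP_SpawnArea is a spawn volume that drops fruit actors at random positions inside its Box component.
; Its DoSpawn event runs a three-step sequence, spawning one actor from each of three class variables.
; Each spawn picks its own random point around the box center, using half the scaled extent, so fruit lands only within the inner region.
; Nothing in this Blueprint calls DoSpawn, and a leftover loop is unconnected.
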(event `Do Spawn`
  (bind _box (`self.Box`))
  (bind _box_2 (`self.Box`))
  (bind _box_3 (`self.Box`))
  ; 시퀀스: 순서대로 하나씩 진행
  (`|ExecutionSequence`
    (:`then_0`
      ; Spawn Actor Area에서 과일1개가 스폰된다.
      (`|SpawnActorFromClass` (`self.SpawnAcrtor Area`) (`KismetMathLibrary.MakeTransform` (`KismetMathLibrary.RandomPointInBoundingBox` (`SceneComponent.K2_GetComponentLocation` _box_2) (/ (`BoxComponent.GetScaledBoxExtent` _box_2) 2.0))) "Undefined" "MultiplyWithRoot" null null))
    (:`then_1`
      ; Spawn Actor Area1에서 과일1개가 스폰된다.
      (`|SpawnActorFromClass` (`self.SpawnAcrtor Area1`) (`KismetMathLibrary.MakeTransform` (`KismetMathLibrary.RandomPointInBoundingBox` (`SceneComponent.K2_GetComponentLocation` _box_3) (/ (`BoxComponent.GetScaledBoxExtent` _box_3) 2.0))) "Undefined" "MultiplyWithRoot" null null))
    (:`then_2`
      ; Spawn Actor Area2에서 과일1개가 스폰된다.
      (`|SpawnActorFromClass` (`self.SpawnAcrtor Area2`) (`KismetMathLibrary.MakeTransform` (`KismetMathLibrary.RandomPointInBoundingBox` (`SceneComponent.K2_GetComponentLocation` _box) (/ (`BoxComponent.GetScaledBoxExtent` _box) 2.0))) "Undefined" "MultiplyWithRoot" null null))))

(fn `UserConstructionScript`)