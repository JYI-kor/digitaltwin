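; BP_LeftRight is an actor that slides its Box component back and forth along relative X between two fixed limits.
; While IsPlay is true, Tick calls MoveRight or MoveLeft, flipping a direction flag (오른쪽이동인가) at either end.
; Movement is a fixed step per frame, so speed depends on frame rate.
; PlayAndStop sets IsPlay and always returns false, whereas the PlayandStop1 event writes its input to the direction flag instead.
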(event `self.ReceiveTick`
  (params (DeltaSeconds :type "Float (single-precision)"))
  (if (`self.Is Play`)
    (if (`self.오른쪽 이동인가?`)
      (`self.MoveRight`)
      (if (>= (`self.X의 위치`) 500.0)
        (set `self.오른쪽 이동인가?` false))
      (else
        (`self.MoveLeft`)
        (if (<= (`self.X의 위치`) 0.0)
          (set `self.오른쪽 이동인가?` true))))))

(event `Play and Stop1`
  (params (`Is play` :type Boolean))
  (set `self.오른쪽 이동인가?` `Is play`))

(fn `MoveLeft`
  ; 왼쪽으로 이동한다.
  ;; X의 위치에 10을 뺀다.
  (set `self.X의 위치` (- (`self.X의 위치`) 10.0))
  ;; Box의 상대좌표 X를 "X의 위치"값으로 변경한다.
  (`SceneComponent.K2_SetRelativeLocation` (`self.Box`) (`KismetMathLibrary.MakeVector` (`self.X의 위치`)) false false))

(fn `MoveRight`
  ; 오른쪽으로 이동한다.
  ;; X의 위치에 10을 더한다.
  (set `self.X의 위치` (+ (`self.X의 위치`) 10.0))
  ;; Box의 상대좌표 X를 "X의 위치"값으로 변경한다.
  (`SceneComponent.K2_SetRelativeLocation` (`self.Box`) (`KismetMathLibrary.MakeVector` (`self.X의 위치`)) false false))

(fn `Play and Stop`
  (params (IsPlay :type Boolean))
  (returns (bResult :type Boolean))
  (set `self.Is Play` IsPlay)
  (return false))

(fn `UserConstructionScript`)