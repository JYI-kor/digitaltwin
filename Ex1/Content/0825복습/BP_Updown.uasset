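; BP_Updown is an actor that bobs its Cone component vertically between relative Z 0 and 500 while IsPlay is true.
; Tick checks the IsMoveUP flag, calls MoveUp or MoveDown, and flips the flag at each limit.
; Each move is a fixed per-frame step without delta time, so speed depends on frame rate.
; A PlayandStop event and a similarly named function both set IsPlay to toggle the motion.
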(event `self.ReceiveTick`
  (params (DeltaSeconds :type "Float (single-precision)"))
  (if (`self.Is Play`)
    (if (`self.IsMoveUP`)
      (`self.Move Up`)
      (if (>= (`self.LocZ`) 500.0)
        (set `self.IsMoveUP` false))
      (else
        (`self.Move Down`)
        (if (<= (`self.LocZ`) 0.0)
          (set `self.IsMoveUP` true))))))

(event `PlayandStop`
  (params (`Is play` :type Boolean))
  (set `self.Is Play` `Is play`))

(fn `Move Down`
  ; 아래로 이동한다
  ;; Z에 10을 뺀다.
  (set `self.LocZ` (- (`self.LocZ`) 10.0))
  ;; Cone의 상대좌표 Z를 "Loc Z"로 변경한다.
  (`SceneComponent.K2_SetRelativeLocation` (`self.Cone`) (`KismetMathLibrary.MakeVector` 0.0 0.0 (`self.LocZ`)) false false))

(fn `Move Up`
  ; 위로 이동한다
  ;; z에 10 더한다.
  (set `self.LocZ` (+ (`self.LocZ`) 10.0))
  ;; Cone의 상대좌표 Z를 "Loc Z"로 변경한다.
  (`SceneComponent.K2_SetRelativeLocation` (`self.Cone`) (`KismetMathLibrary.MakeVector` 0.0 0.0 (`self.LocZ`)) false false))

(fn `Play and Stop`
  (params (IsPlay :type Boolean))
  (returns (bResult :type Boolean))
  (set `self.Is Play` IsPlay)
  (return false))

(fn `UserConstructionScript`)