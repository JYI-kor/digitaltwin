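; BP_MoveRect is an actor that moves its Cube around a rectangular loop in the local XZ plane while playing.
; Tick switches on a MoveType state and calls one of four directional functions, each stepping the Cube by a fixed per-frame offset, independent of delta time.
; Each function advances the state at its boundary, cycling right, up, left, down.
; An event and a similar function set the Isplay flag to start or stop motion.
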(event `self.ReceiveTick`
  (params (DeltaSeconds :type "Float (single-precision)"))
  (if (`self.Isplay`)
    (switch `/Game/0825복습/ENUM_MoveType` (`self.MoveType`)
      (:`NewEnumerator0`
        (`self.Move Right`))
      (:`NewEnumerator1`
        (`self.Move Up`))
      (:`NewEnumerator2`
        (`self.Move Left`))
      (:`NewEnumerator3`
        (`self.Move Down`)))))

(event `Play and Stop1`
  (params (`Is play` :type Boolean))
  (set `self.Isplay` `Is play`))

(fn `Move Down`
  (bind (_relativelocation_x _relativelocation_y _relativelocation_z) (`KismetMathLibrary.BreakVector` (`SceneComponent.RelativeLocation` (`self.Cube`))))
  ; 아래로 이동한다
  (`SceneComponent.K2_AddRelativeLocation` (`self.Cube`) (0.0 0.0 -25.0) false false)
  (if (< _relativelocation_z 0.0)
    (set `self.MoveType` "NewEnumerator0")))

(fn `Move Left`
  (bind _relativelocation_x (`KismetMathLibrary.BreakVector` (`SceneComponent.RelativeLocation` (`self.Cube`))))
  ; 왼쪽으로 이동한다
  (`SceneComponent.K2_AddRelativeLocation` (`self.Cube`) (-25.0 0.0 0.0) false false)
  (if (< _relativelocation_x 0.0)
    (set `self.MoveType` "NewEnumerator3")))

(fn `Move Right`
  (bind _relativelocation_x (`KismetMathLibrary.BreakVector` (`SceneComponent.RelativeLocation` (`self.Cube`))))
  ; 오른쪽으로 이동한다
  (`SceneComponent.K2_AddRelativeLocation` (`self.Cube`) (25.0 0.0 0.0) false false)
  (if (> _relativelocation_x 500.0)
    (set `self.MoveType` "NewEnumerator1")))

(fn `Move Up`
  (bind (_relativelocation_x _relativelocation_y _relativelocation_z) (`KismetMathLibrary.BreakVector` (`SceneComponent.RelativeLocation` (`self.Cube`))))
  ; 위쪽으로 이동한다
  (`SceneComponent.K2_AddRelativeLocation` (`self.Cube`) (0.0 0.0 25.0) false false)
  (if (> _relativelocation_z 500.0)
    (set `self.MoveType` "NewEnumerator2")))

(fn `Play and Stop`
  (params (IsPlay :type Boolean))
  (returns (bResult :type Boolean))
  (set `self.Isplay` IsPlay)
  (return false))

(fn `UserConstructionScript`)