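; BP_CountBox is a counter for a collect game that shows a running Count on a TextRender component.
; The DoGet event increments Count by one and DoGet1 decrements it by one.
; Both events call ShowCount to convert the value to text and refresh the display, which also runs at BeginPlay.
; A separate AddCount function only prints a string and leaves Count untouched.
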(event `self.ReceiveBeginPlay`
  (`self.ShowCount`))

(event `/Game/0827연습/ColletGame/BPI_Fruit.DoGet`
  ; Count가 1씩 증가한다.
  (set `self.Count` (+ (`self.Count`) 1))
  (`self.ShowCount`))

(event `/Game/0827연습/ColletGame/BPI_Fruit.DoGet1`
  ; Count가 1씩 감소한다.
  (set `self.Count` (- (`self.Count`) 1))
  (`self.ShowCount`))

(fn `Add Count`
  (`KismetSystemLibrary.PrintString` "Hello"))

(fn `ShowCount`
  (`TextRenderComponent.K2_SetText` (`self.TextRender`) (`KismetTextLibrary.Conv_IntToText` (`self.Count`))))

(fn `UserConstructionScript`)