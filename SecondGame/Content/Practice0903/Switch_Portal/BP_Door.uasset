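; BP_Door is a level-exit portal whose door mesh is hidden at BeginPlay and loads LVl_ThirdPerson on any overlap.
; CoinCheck shows the door when no live BP_Coin2 actors remain, while OverlapBox shows it when CountBox's count equals ten.
; BeginPlay binds to CountBox's OpenDoor dispatcher.
; Only visibility is toggled, and the overlap handler does not check it before loading.
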(event `self.ReceiveBeginPlay`
  (`SceneComponent.SetVisibility` (`self.Door`) false false)
  (add `/Game/Practice0903/Switch_Portal/BP_CountBox.NewEventDispatcher_Open Door` (`self.CountBox`) (`|CreateDelegate` :!event `Overlap BOx`)))

(event `self.Door.OnComponentBeginOverlap`
  (params (OverlappedComponent :type "PrimitiveComponent Object Reference") (OtherActor :type "Actor Object Reference") (OtherComp :type "PrimitiveComponent Object Reference") (OtherBodyIndex :type Integer) (bFromSweep :type Boolean) (SweepResult :type "HitResult Structure (by ref)"))
  (`GameplayStatics.OpenLevel` "LVl_ThirdPerson"))

(fn `Box Is 10`
  (returns (`Box Is 10` :type Boolean))
  (if (== (`/Game/Practice0903/Switch_Portal/BP_CountBox.Count` (`self.CountBox`)) 10)
    (return true)
    (else
      (return false))))

(fn `Coin Check`
  (`SceneComponent.SetVisibility` (`self.Door`) (== (`self.Remain Coin`) 0) false))

(fn `Overlap Box`
  (`SceneComponent.SetVisibility` (`self.Door`) (`self.Box Is 10`) false))

(fn `Remain Coin`
  (returns (Remain :type Integer))
  (locals (Coin :type Integer))
  (bind _outactors (`GameplayStatics.GetAllActorsOfClass` "/Game/Practice0903/GetCoin_Second/BP_Coin2.BP_Coin2_C"))
  (for _array_element _outactors
    (if (not (`self.IsActorBeingDestroyed` _array_element))
      (set `local.Coin` (+ (`local.Coin`) 1))))
  (return (`local.Coin`)))

(fn `UserConstructionScript`)