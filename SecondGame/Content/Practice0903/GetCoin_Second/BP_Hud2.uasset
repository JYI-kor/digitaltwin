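; BP_Hud2 is a coin-collection HUD that creates the HudWidget2 widget and displays how many BP_Coin2 actors remain in the level.
; On BeginPlay it binds a handler to every coin's get-coin event dispatcher, then pushes the initial count to the widget.
; The count comes from scanning all BP_Coin2 actors and skipping those being destroyed.
; A separate GetCoin function sends a fixed zero to the widget.
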(event `self.ReceiveBeginPlay`
  (bind _returnvalue (`|CreateWidget` "/Game/Practice0903/GetCoin_Second/HudWidget2.HudWidget2_C"))
  (bind _output_get (set `self.HudWidget2` _returnvalue))
  (`UserWidget.AddToViewport` _output_get 0)
  ; 월드내 존재하는 클래스에 해당하는 액터를 부른다
  (bind _outactors (`GameplayStatics.GetAllActorsOfClass` "/Game/Practice0903/GetCoin_Second/BP_Coin2.BP_Coin2_C"))
  (for _array_element _outactors
    (add `/Game/Practice0903/GetCoin_Second/BP_Coin2.NewEventDispatcher_Get Coin` _array_element (`|CreateDelegate` :!event `HudWidget Show Coin`)))
  (`self.HudWidget Show Coin`))

(fn `Get Coin`
  (`/Game/Practice0903/GetCoin_Second/HudWidget2.Show Coin` (`self.HudWidget2`) 0))

(fn `HudWidget Show Coin`
  (`/Game/Practice0903/GetCoin_Second/HudWidget2.Show Coin` (`self.HudWidget2`) (`self.Remain Coin`)))

(fn `Remain Coin`
  (returns (Remain :type Integer))
  (locals (Coin :type Integer))
  (bind _outactors (`GameplayStatics.GetAllActorsOfClass` "/Game/Practice0903/GetCoin_Second/BP_Coin2.BP_Coin2_C"))
  (for _array_element _outactors
    (if (not (`self.IsActorBeingDestroyed` _array_element))
      (set `local.Coin` (+ (`local.Coin`) 1))))
  (return (`local.Coin`)))

(fn `UserConstructionScript`)