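; BP_Coin2 is a collectible coin pickup that spins by a fixed rotation step every tick, independent of delta time.
; When a Character overlaps the Coin component, it casts through that character's PlayerController to BP_Hud2 and calls GetCoin on the HUD directly.
; It then destroys itself and afterwards fires its GetCoin event dispatcher.
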(event `self.ReceiveTick`
  (params (DeltaSeconds :type "Float (single-precision)"))
  (`SceneComponent.K2_AddRelativeRotation` (`self.Coin`) (struct :`Yaw` 5.0) false false))

(event `self.Coin.OnComponentBeginOverlap`
  (params (OverlappedComponent :type "PrimitiveComponent Object Reference") (OtherActor :type "Actor Object Reference") (OtherComp :type "PrimitiveComponent Object Reference") (OtherBodyIndex :type Integer) (bFromSweep :type Boolean) (SweepResult :type "HitResult Structure (by ref)"))
  (bind _ascharacter (cast `Character` OtherActor))
  (bind _asplayer_controller (cast `PlayerController` (`Pawn.GetController` _ascharacter)))
  (bind _asbp_hud_2 (cast `/Game/Practice0903/GetCoin_Second/BP_Hud2` (`PlayerController.GetHUD` _asplayer_controller)))
  (`/Game/Practice0903/GetCoin_Second/BP_Hud2.Get Coin` _asbp_hud_2)
  (`self.K2_DestroyActor`)
  (`self.NewEventDispatcher_Get Coin`))

(fn `UserConstructionScript`)