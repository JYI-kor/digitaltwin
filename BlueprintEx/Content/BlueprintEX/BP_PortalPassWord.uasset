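; BP_PortalPassWord is a password lock that shows its Sphere only while a set of counting boxes matches the code.
; On BeginPlay it sets the initial visibility and binds to the F-press dispatcher of every box in CountingBoxes, apparently to re-run the check on each press.
; IsAllBox9 compares each box's Count with the PassWord entry at the same index, despite its name suggesting a fixed 9.
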(event `self.ReceiveBeginPlay`
  (`SceneComponent.SetVisibility` (`self.Sphere`) (`self.Is All Box9`) false)
  ; Counting Box Binding
  (for _array_element (`self.Counting Boxes`)
    (add `/Game/BlueprintEX/BP_CountingBox.NewEventDispatcher_F Press` _array_element (`|CreateDelegate` :!event ` Func_Press F Tolggle`))))

(fn ` Func_Press F Tolggle`
  (`SceneComponent.SetVisibility` (`self.Sphere`) (`self.Is All Box9`) false))

(fn `Is All Box9`
  (returns (`All Box 9` :type Boolean))
  (for (_array_element _array_index) (`self.Counting Boxes`)
    (if (not (== (`/Game/BlueprintEX/BP_CountingBox.Count` _array_element) (`|GetArrayItem` (`self.PassWord`) _array_index)))
      (return false)))
  (return true))

(fn `UserConstructionScript`)