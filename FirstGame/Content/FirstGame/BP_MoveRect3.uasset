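; BP_MoveRect3 is an actor that moves its Sphere component continuously around a rectangular path in the local X-Z plane.
; Each Tick switches on the MoveType3 enum as a simple state machine, offsetting the sphere up, right, down or left.
; When the relative location crosses that side's limit, the state advances to the next direction.
; Movement is a fixed step per frame without delta time, so speed depends on frame rate.
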(event `self.ReceiveTick`
  (params (DeltaSeconds :type "Float (single-precision)"))
  (bind _relativelocation_x (`KismetMathLibrary.BreakVector` (`SceneComponent.RelativeLocation` (`self.Sphere`))))
  (bind (_relativelocation_x_2 _relativelocation_y _relativelocation_z) (`KismetMathLibrary.BreakVector` (`SceneComponent.RelativeLocation` (`self.Sphere`))))
  (bind _relativelocation_x_3 (`KismetMathLibrary.BreakVector` (`SceneComponent.RelativeLocation` (`self.Sphere`))))
  (bind (_relativelocation_x_4 _relativelocation_y_2 _relativelocation_z_2) (`KismetMathLibrary.BreakVector` (`SceneComponent.RelativeLocation` (`self.Sphere`))))
  (switch `/Game/FirstGame/ENUM_MoveType3` (`self.MoveType3`)
    (:`NewEnumerator0`
      ; 위로 움직인다.
      (set `self.MoveType3` "NewEnumerator0")
      (`SceneComponent.K2_AddRelativeLocation` (`self.Sphere`) (0.0 0.0 25.0) false false)
      (if (>= _relativelocation_z_2 500.0)
        (set `self.MoveType3` "NewEnumerator1")))
    (:`NewEnumerator1`
      ; 오른쪽으로 움직인다.
      (set `self.MoveType3` "NewEnumerator1")
      (`SceneComponent.K2_AddRelativeLocation` (`self.Sphere`) (25.0 0.0 0.0) false false)
      (if (>= _relativelocation_x 500.0)
        (set `self.MoveType3` "NewEnumerator2")))
    (:`NewEnumerator2`
      ; 아래로 움직인다
      (set `self.MoveType3` "NewEnumerator2")
      (`SceneComponent.K2_AddRelativeLocation` (`self.Sphere`) (0.0 0.0 -25.0) false false)
      (if (<= _relativelocation_z 0.0)
        (set `self.MoveType3` "NewEnumerator3")))
    (:`NewEnumerator3`
      ; 왼쪽으로 움직인다
      (set `self.MoveType3` "NewEnumerator3")
      (`SceneComponent.K2_AddRelativeLocation` (`self.Sphere`) (-25.0 0.0 0.0) false false)
      (if (<= _relativelocation_x_3 0.0)
        (set `self.MoveType3` "NewEnumerator0")))))

(fn `UserConstructionScript`)