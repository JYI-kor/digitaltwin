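; BP_MoveRect2 is an actor Blueprint that loops its Sphere component around a square path in the local X-Z plane.
; Each Tick, a switch on the Movetype2 state steps the X or Z position variable by a fixed amount and sets the sphere's relative location.
; Reaching each boundary advances the state through Left, Down, Right and Up.
; Movement is per frame without delta time, so speed depends on frame rate.
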(event `self.ReceiveTick`
  (params (DeltaSeconds :type "Float (single-precision)"))
  (switch `/Game/FirstGame/BP_0821/ENUM_MoveType2` (`self.Movetype2`)
    (:`NewEnumerator0`
      ; 왼쪽으로 이동한다.
      (bind _output_get (set `self.Positon of X` (- (`self.Positon of X`) 25.0)))
      (`SceneComponent.K2_SetRelativeLocation` (`self.Sphere`) (`KismetMathLibrary.MakeVector` _output_get 0.0 (`self.Positon of Z`)) false false)
      (if (<= (`self.Positon of X`) -500.0)
        (set `self.Movetype2` "NewEnumerator1")))
    (:`NewEnumerator1`
      ; 아래로 이동한다
      (bind _output_get_2 (set `self.Positon of Z` (- (`self.Positon of Z`) 25.0)))
      (`SceneComponent.K2_SetRelativeLocation` (`self.Sphere`) (`KismetMathLibrary.MakeVector` (`self.Positon of X`) 0.0 _output_get_2) false false)
      (if (<= (`self.Positon of Z`) -500.0)
        (set `self.Movetype2` "NewEnumerator2")))
    (:`NewEnumerator2`
      ; 오른쪽으로 이동한다
      (bind _output_get_3 (set `self.Positon of X` (+ (`self.Positon of X`) 25.0)))
      (`SceneComponent.K2_SetRelativeLocation` (`self.Sphere`) (`KismetMathLibrary.MakeVector` _output_get_3 0.0 (`self.Positon of Z`)) false false)
      (if (>= (`self.Positon of X`) 0.0)
        (set `self.Movetype2` "NewEnumerator3")))
    (:`NewEnumerator3`
      ; 위로 이동한다
      (bind _output_get_4 (set `self.Positon of Z` (+ (`self.Positon of Z`) 25.0)))
      (`SceneComponent.K2_SetRelativeLocation` (`self.Sphere`) (`KismetMathLibrary.MakeVector` (`self.Positon of X`) 0.0 _output_get_4) false false)
      (if (>= (`self.Positon of Z`) 0.0)
        (set `self.Movetype2` "NewEnumerator0")))))

(fn `UserConstructionScript`)