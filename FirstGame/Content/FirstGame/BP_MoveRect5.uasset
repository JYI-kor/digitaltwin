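; Actor that moves its Sphere component back and forth along a two-step staircase path in the X-Z plane, looping continuously.
; Each Tick switches on the MoveR enum, an eight-state machine that nudges the sphere's relative location by a fixed per-frame step, independent of delta time.
; Relative-position thresholds advance the state, climbing up and right, then retracing the same steps left and down to restart.
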(event `self.ReceiveTick`
  (params (DeltaSeconds :type "Float (single-precision)"))
  (bind _relativelocation_x (`KismetMathLibrary.BreakVector` (`SceneComponent.RelativeLocation` (`self.Sphere`))))
  (bind _relativelocation_x_2 (`KismetMathLibrary.BreakVector` (`SceneComponent.RelativeLocation` (`self.Sphere`))))
  (bind _relativelocation_x_3 (`KismetMathLibrary.BreakVector` (`SceneComponent.RelativeLocation` (`self.Sphere`))))
  (bind (_relativelocation_x_4 _relativelocation_y _relativelocation_z) (`KismetMathLibrary.BreakVector` (`SceneComponent.RelativeLocation` (`self.Sphere`))))
  (bind (_relativelocation_x_5 _relativelocation_y_2 _relativelocation_z_2) (`KismetMathLibrary.BreakVector` (`SceneComponent.RelativeLocation` (`self.Sphere`))))
  (bind (_relativelocation_x_6 _relativelocation_y_3 _relativelocation_z_3) (`KismetMathLibrary.BreakVector` (`SceneComponent.RelativeLocation` (`self.Sphere`))))
  (bind (_relativelocation_x_7 _relativelocation_y_4 _relativelocation_z_4) (`KismetMathLibrary.BreakVector` (`SceneComponent.RelativeLocation` (`self.Sphere`))))
  (bind _relativelocation_x_8 (`KismetMathLibrary.BreakVector` (`SceneComponent.RelativeLocation` (`self.Sphere`))))
  (switch `/Game/FirstGame/ENUM_MoveType5` (`self.MoveR`)
    (:`NewEnumerator0`
      ; 위쪽으로 이동한다.
      (set `self.MoveR` "NewEnumerator0")
      (`SceneComponent.K2_AddRelativeLocation` (`self.Sphere`) (0.0 0.0 5.0) false false)
      (if (>= _relativelocation_z_4 100.0)
        (set `self.MoveR` "NewEnumerator1")))
    (:`NewEnumerator1`
      ; 오른쪽으로 이동한다.
      (set `self.MoveR` "NewEnumerator1")
      (`SceneComponent.K2_AddRelativeLocation` (`self.Sphere`) (5.0 0.0 0.0) false false)
      (if (>= _relativelocation_x 100.0)
        (set `self.MoveR` "NewEnumerator2")))
    (:`NewEnumerator2`
      ; 위쪽으로 이동한다.
      (set `self.MoveR` "NewEnumerator2")
      (`SceneComponent.K2_AddRelativeLocation` (`self.Sphere`) (0.0 0.0 5.0) false false)
      (if (>= _relativelocation_z_3 200.0)
        (set `self.MoveR` "NewEnumerator3")))
    (:`NewEnumerator3`
      ; 오른쪽으로 이동한다.
      (set `self.MoveR` "NewEnumerator3")
      (`SceneComponent.K2_AddRelativeLocation` (`self.Sphere`) (5.0 0.0 0.0) false false)
      (if (>= _relativelocation_x_2 200.0)
        (set `self.MoveR` "NewEnumerator4")))
    (:`NewEnumerator4`
      ; 왼쪽으로 이동한다
      (set `self.MoveR` "NewEnumerator4")
      (`SceneComponent.K2_AddRelativeLocation` (`self.Sphere`) (-5.0 0.0 0.0) false false)
      (if (<= _relativelocation_x_3 100.0)
        (set `self.MoveR` "NewEnumerator5")))
    (:`NewEnumerator5`
      ; 아래쪽으로 이동한다.
      (set `self.MoveR` "NewEnumerator5")
      (`SceneComponent.K2_AddRelativeLocation` (`self.Sphere`) (0.0 0.0 -5.0) false false)
      (if (<= _relativelocation_z_2 100.0)
        (set `self.MoveR` "NewEnumerator6")))
    (:`NewEnumerator6`
      ; 왼쪽으로 이동한다.
      (set `self.MoveR` "NewEnumerator6")
      (`SceneComponent.K2_AddRelativeLocation` (`self.Sphere`) (-5.0 0.0 0.0) false false)
      (if (<= _relativelocation_x_8 0.0)
        (set `self.MoveR` "NewEnumerator7")))
    (:`NewEnumerator7`
      ; 아래쪽으로 이동한다.
      (set `self.MoveR` "NewEnumerator7")
      (`SceneComponent.K2_AddRelativeLocation` (`self.Sphere`) (0.0 0.0 -5.0) false false)
      (if (<= _relativelocation_z 0.0)
        (set `self.MoveR` "NewEnumerator0")))))

(fn `UserConstructionScript`)