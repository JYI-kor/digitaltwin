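; BP_Canon1 is a cannon actor that automatically fires BP_CanonBall projectiles while switched on.
; Each PressF event flips a toggle that starts or clears a looping one-second timer, bound by function name to Do Shoot.
; Do Shoot spawns a cannonball at the world location and rotation of the Arrow component, which serves as the muzzle.
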(event `self.Press F`
  (bind _output_get (set `self.Toggle` (not (`self.Toggle`))))
  (if _output_get
    (`KismetSystemLibrary.K2_SetTimer` null "Do Shoot" 1.0 true)
    (else
      (`KismetSystemLibrary.K2_ClearTimer` null "Do Shoot"))))

(fn `Do Shoot`
  (bind _arrow (`self.Arrow`))
  (`|SpawnActorFromClass` "/Game/FirstGame/BP_0828/BP_CanonBall.BP_CanonBall_C" (`KismetMathLibrary.MakeTransform` (`SceneComponent.K2_GetComponentLocation` _arrow) (`SceneComponent.K2_GetComponentRotation` _arrow)) "Undefined" "MultiplyWithRoot" null null))

(fn `UserConstructionScript`)