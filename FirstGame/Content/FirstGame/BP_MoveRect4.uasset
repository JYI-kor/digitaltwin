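; BP_MoveRect4 is a Blueprint that moves its Plane component back and forth along an L-shaped path in the X-Z plane.
; Each Tick switches on the MoveType4 enum state, cycling Right, Up, Down and Left as relative-location limits are reached.
; Movement uses a fixed, unswept offset per tick without delta-time scaling, so speed depends on frame rate.
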(event `self.ReceiveTick`
  (params (DeltaSeconds :type "Float (single-precision)"))
  (bind _relativelocation_x (`KismetMathLibrary.BreakVector` (`SceneComponent.RelativeLocation` (`self.Plane`))))
  (bind (_relativelocation_x_2 _relativelocation_y _relativelocation_z) (`KismetMathLibrary.BreakVector` (`SceneComponent.RelativeLocation` (`self.Plane`))))
  (bind (_relativelocation_x_3 _relativelocation_y_2 _relativelocation_z_2) (`KismetMathLibrary.BreakVector` (`SceneComponent.RelativeLocation` (`self.Plane`))))
  (bind _relativelocation_x_4 (`KismetMathLibrary.BreakVector` (`SceneComponent.RelativeLocation` (`self.Plane`))))
  (switch `/Game/FirstGame/ENUM_MoveType4` (`self.MoveType4`)
    (:`NewEnumerator0`
      ; 오른쪽으로 움직인다.
      (set `self.MoveType4` "NewEnumerator0")
      (`SceneComponent.K2_AddRelativeLocation` (`self.Plane`) (25.0 0.0 0.0) false false)
      (if (>= _relativelocation_x 500.0)
        (set `self.MoveType4` "NewEnumerator1")))
    (:`NewEnumerator1`
      ; 위로 움직인다.
      (set `self.MoveType4` "NewEnumerator1")
      (`SceneComponent.K2_AddRelativeLocation` (`self.Plane`) (0.0 0.0 25.0) false false)
      (if (>= _relativelocation_z 500.0)
        (set `self.MoveType4` "NewEnumerator2")))
    (:`NewEnumerator2`
      ; 아래로 움직인다
      (set `self.MoveType4` "NewEnumerator2")
      (`SceneComponent.K2_AddRelativeLocation` (`self.Plane`) (0.0 0.0 -25.0) false false)
      (if (<= _relativelocation_z_2 0.0)
        (set `self.MoveType4` "NewEnumerator3")))
    (:`NewEnumerator3`
      ; 왼쪽으로 움직인다
      (set `self.MoveType4` "NewEnumerator3")
      (`SceneComponent.K2_AddRelativeLocation` (`self.Plane`) (-25.0 0.0 0.0) false false)
      (if (<= _relativelocation_x_4 0.0)
        (set `self.MoveType4` "NewEnumerator0")))))

(fn `UserConstructionScript`)