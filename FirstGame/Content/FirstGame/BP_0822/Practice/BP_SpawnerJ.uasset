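; BP_SpawnerJ is a practice spawner actor that drops BP_Ball actors at its own transform, one per call.
; Its custom event 공떨구기 (drop ball) increments a float counter before each spawn and stops at a fixed cap, with no decrement in this graph.
; The construction script writes the actor's display name to a TextRender, labeling each spawner.
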(event `공 떨구기`
  ; 볼의 갯수가 9.5개 이상인가?
  (if (not (>= (`self.number of ball`) 9.5))
    ; 볼을 1개씩 스폰한다.
    (set `self.number of ball` (+ (`self.number of ball`) 1.0))
    (`|SpawnActorFromClass` "/Game/FirstGame/BP_0822/Practice/BP_Ball.BP_Ball_C" (`self.GetTransform`) "Undefined" "MultiplyWithRoot" null null)))

(fn `UserConstructionScript`
  (`TextRenderComponent.K2_SetText` (`self.TextRender`) (`KismetTextLibrary.Conv_StringToText` (`KismetSystemLibrary.GetDisplayName` self))))