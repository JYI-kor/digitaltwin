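; BP_Switch1 is an overlap-triggered switch that drives a list of linked actors through interfaces.
; When its Cube is entered, each actor in Actors receives PlayAndStop(true) through BPI_PlayStop, or otherwise DoSpawn through BPI_Spawn.
; Leaving the Cube sends PlayAndStop(false) to the BPI_PlayStop actors.
; The construction script labels the switch with its display name, and its own Play and Stop function is a stub returning false.
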(event `self.Cube.OnComponentBeginOverlap`
  (params (OverlappedComponent :type "PrimitiveComponent Object Reference") (OtherActor :type "Actor Object Reference") (OtherComp :type "PrimitiveComponent Object Reference") (OtherBodyIndex :type Integer) (bFromSweep :type Boolean) (SweepResult :type "HitResult Structure (by ref)"))
  (for _array_element (`self.Actors`)
    (bind _asbpi_play_stop (cast `/Game/FirstGame/BP_0827/BPI_PlayStop` _array_element)
      (:`then`
        (`/Game/FirstGame/BP_0827/BPI_PlayStop.Play and Stop` _asbpi_play_stop true))
      (:`CastFailed`
        (bind _asbpi_spawn (cast `/Game/FirstGame/BP_0827/BPI_Spawn` _array_element))
        (`/Game/FirstGame/BP_0827/BPI_Spawn.DoSpawn` _asbpi_spawn)))))

(event `self.Cube.OnComponentEndOverlap`
  (params (OverlappedComponent :type "PrimitiveComponent Object Reference") (OtherActor :type "Actor Object Reference") (OtherComp :type "PrimitiveComponent Object Reference") (OtherBodyIndex :type Integer))
  (for _array_element (`self.Actors`)
    (bind _asbpi_play_stop (cast `/Game/FirstGame/BP_0827/BPI_PlayStop` _array_element))
    (`/Game/FirstGame/BP_0827/BPI_PlayStop.Play and Stop` _asbpi_play_stop false)))

(fn `Play and Stop`
  (params (`Is Play` :type Boolean))
  (returns (bResult :type Boolean))
  (return false))

(fn `UserConstructionScript`
  (`TextRenderComponent.K2_SetText` (`self.TextRender`) (`KismetTextLibrary.Conv_StringToText` (`KismetSystemLibrary.GetDisplayName` self))))