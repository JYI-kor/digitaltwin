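; Blueprint that moves its Cube component around a square path in the X-Z plane while IsPlay is true.
; Each Tick switches on the MoveType enum (Right, Up, Left, Down) and nudges the cube's relative location by a fixed step.
; Crossing that side's bound advances MoveType to the next direction, forming a looping state machine.
; The step is per frame, not scaled by delta time, so speed depends on frame rate.
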(event `self.ReceiveTick`
  (params (DeltaSeconds :type "Float (single-precision)"))
  (bind _relativelocation_x (`KismetMathLibrary.BreakVector` (`SceneComponent.RelativeLocation` (`self.Cube`))))
  (bind (_relativelocation_x_2 _relativelocation_y _relativelocation_z) (`KismetMathLibrary.BreakVector` (`SceneComponent.RelativeLocation` (`self.Cube`))))
  (bind _relativelocation_x_3 (`KismetMathLibrary.BreakVector` (`SceneComponent.RelativeLocation` (`self.Cube`))))
  (bind (_relativelocation_x_4 _relativelocation_y_2 _relativelocation_z_2) (`KismetMathLibrary.BreakVector` (`SceneComponent.RelativeLocation` (`self.Cube`))))
  (if (`self.IsPlay`)
    (switch `/Game/FirstGame/BP_0821/ENUM_MoveType` (`self.MoveType`)
      (:`NewEnumerator0`
        ; 오른쪽으로 이동한다
        (set `self.MoveType` "NewEnumerator0")
        (`SceneComponent.K2_AddRelativeLocation` (`self.Cube`) (25.0 0.0 0.0) false false)
        (if (> _relativelocation_x 500.0)
          (set `self.MoveType` "NewEnumerator1")))
      (:`NewEnumerator1`
        ; 위쪽으로 이동한다
        (set `self.MoveType` "NewEnumerator1")
        (`SceneComponent.K2_AddRelativeLocation` (`self.Cube`) (0.0 0.0 25.0) false false)
        (if (> _relativelocation_z 500.0)
          (set `self.MoveType` "NewEnumerator2")))
      (:`NewEnumerator2`
        ; 왼쪽으로 이동한다
        (set `self.MoveType` "NewEnumerator2")
        (`SceneComponent.K2_AddRelativeLocation` (`self.Cube`) (-25.0 0.0 0.0) false false)
        (if (< _relativelocation_x_3 0.0)
          (set `self.MoveType` "NewEnumerator3")))
      (:`NewEnumerator3`
        ; 아래로 이동한다
        (set `self.MoveType` "NewEnumerator3")
        (`SceneComponent.K2_AddRelativeLocation` (`self.Cube`) (0.0 0.0 -25.0) false false)
        (if (< _relativelocation_z_2 0.0)
          (set `self.MoveType` "NewEnumerator0"))))))

(fn `UserConstructionScript`)