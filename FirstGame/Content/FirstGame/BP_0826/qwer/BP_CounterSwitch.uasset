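; BP_CounterSwitch is an overlap-triggered switch that shows a wrapping single-digit counter and toggles the actors in its Actors array.
; Each overlap on Cube1 increments Count, resets it past nine, updates the TextRender, then branches on parity.
; Chained casts start the supported mover actors and trigger spawners on odd counts.
; Even counts stop only the movers, through either IsPlay flags or DoStop calls.
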(event `self.ReceiveBeginPlay`
  ; 시작할 때 Count값을 Text Render에 표시.
  (`TextRenderComponent.K2_SetText` (`self.TextRender`) (`KismetTextLibrary.Conv_IntToText` (`self.Count`) false true 1 244)))

(event `self.cube1.OnComponentBeginOverlap`
  (params (OverlappedComponent :type "PrimitiveComponent Object Reference") (OtherActor :type "Actor Object Reference") (OtherComp :type "PrimitiveComponent Object Reference") (OtherBodyIndex :type Integer) (bFromSweep :type Boolean) (SweepResult :type "HitResult Structure (by ref)"))
  (`|ExecutionSequence`
    (:`then_0`
      ; Count증가 표시
      ;; Count를 1증가
      (set `self.Count` (+ (`self.Count`) 1))
      ;; Count가 9보다 크면
      (if (> (`self.Count`) 9)
        ;; Count 0으로 변경
        (set `self.Count` 0))
      ;; Count값을 Text Render에 표시
      (`TextRenderComponent.K2_SetText` (`self.TextRender`) (`KismetTextLibrary.Conv_IntToText` (`self.Count`) false true 1 244)))
    (:`then_1`
      (if (== (mod (`self.Count`) 2) 1)
        ; Count가 홀수일경우
        (for _array_element (`self.Actors`)
          (bind _asbp_left_right_1 (cast `/Game/FirstGame/BP_0826/BP_LeftRight1` _array_element)
            (:`then`
              (set `/Game/FirstGame/BP_0826/BP_LeftRight1.IsPlay` true _asbp_left_right_1))
            (:`CastFailed`
              (bind _asbp_left_right_time_line (cast `/Game/FirstGame/BP_0826/BP_LeftRightTimeLine` _array_element)
                (:`then`
                  (`/Game/FirstGame/BP_0826/BP_LeftRightTimeLine.DoPlay` _asbp_left_right_time_line))
                (:`CastFailed`
                  (bind _asbp_move_rect_1 (cast `/Game/FirstGame/BP_0826/BP_MoveRect1` _array_element)
                    (:`then`
                      (set `/Game/FirstGame/BP_0826/BP_MoveRect1.IsPlay` true _asbp_move_rect_1))
                    (:`CastFailed`
                      (bind _asbp_move_rect_time_line_2 (cast `/Game/FirstGame/BP_0826/BP_MoveRectTimeLine2` _array_element)
                        (:`then`
                          (`/Game/FirstGame/BP_0826/BP_MoveRectTimeLine2.DoPlay` _asbp_move_rect_time_line_2))
                        (:`CastFailed`
                          (bind _asbp_spawn_area_1 (cast `/Game/FirstGame/BP_0826/BP_SpawnArea1` _array_element)
                            (:`then`
                              (`/Game/FirstGame/BP_0826/BP_SpawnArea1.Do Spawn` _asbp_spawn_area_1))
                            (:`CastFailed`
                              (bind _asbp_spawner_1 (cast `/Game/FirstGame/BP_0826/BP_Spawner1` _array_element))
                              (`/Game/FirstGame/BP_0826/BP_Spawner1.DoSpawn` _asbp_spawner_1))))))))))))
        (else
          ; Count가 짝수일경우
          (for _array_element_2 (`self.Actors`)
            (bind _asbp_left_right_1_2 (cast `/Game/FirstGame/BP_0826/BP_LeftRight1` _array_element_2)
              (:`then`
                (set `/Game/FirstGame/BP_0826/BP_LeftRight1.IsPlay` false _asbp_left_right_1_2))
              (:`CastFailed`
                (bind _asbp_left_right_time_line_2 (cast `/Game/FirstGame/BP_0826/BP_LeftRightTimeLine` _array_element_2)
                  (:`then`
                    (`/Game/FirstGame/BP_0826/BP_LeftRightTimeLine.DoStop` _asbp_left_right_time_line_2))
                  (:`CastFailed`
                    (bind _asbp_move_rect_1_2 (cast `/Game/FirstGame/BP_0826/BP_MoveRect1` _array_element_2)
                      (:`then`
                        (set `/Game/FirstGame/BP_0826/BP_MoveRect1.IsPlay` false _asbp_move_rect_1_2))
                      (:`CastFailed`
                        (bind _asbp_move_rect_time_line_2_2 (cast `/Game/FirstGame/BP_0826/BP_MoveRectTimeLine2` _array_element_2))
                        (`/Game/FirstGame/BP_0826/BP_MoveRectTimeLine2.DoStop` _asbp_move_rect_time_line_2_2)))))))))))))

(fn `UserConstructionScript`)