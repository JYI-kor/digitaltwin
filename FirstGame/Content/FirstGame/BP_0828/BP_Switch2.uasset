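; BP_Switch2 is a toggle switch that drives a list of target actors when F is pressed.
; Switching on calls PlayAndStop(true) on targets implementing BPI_PlayStop, otherwise DoSpawn on those implementing BPI_Spawn.
; Switching off calls PlayAndStop(false) on the BPI_PlayStop targets only, so spawn targets get no off signal.
; The construction script writes the switch's display name to its TextRender label.
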(event `self.Press F`
  (bind _output_get (set `self.Toggle` (not (`self.Toggle`))))
  (if _output_get
    (for _array_element (`self.Actors`)
      (bind _asbpi_play_stop (cast `/Game/FirstGame/BP_0827/BPI_PlayStop` _array_element)
        (:`then`
          (`/Game/FirstGame/BP_0827/BPI_PlayStop.Play and Stop` _asbpi_play_stop true))
        (:`CastFailed`
          (bind _asbpi_spawn (cast `/Game/FirstGame/BP_0827/BPI_Spawn` _array_element))
          (`/Game/FirstGame/BP_0827/BPI_Spawn.DoSpawn` _asbpi_spawn))))
    (else
      (for _array_element_2 (`self.Actors`)
        (bind _asbpi_play_stop_2 (cast `/Game/FirstGame/BP_0827/BPI_PlayStop` _array_element_2))
        (`/Game/FirstGame/BP_0827/BPI_PlayStop.Play and Stop` _asbpi_play_stop_2 false)))))

(fn `UserConstructionScript`
  (`TextRenderComponent.K2_SetText` (`self.TextRender`) (`KismetTextLibrary.Conv_StringToText` (`KismetSystemLibrary.GetDisplayName` self))))