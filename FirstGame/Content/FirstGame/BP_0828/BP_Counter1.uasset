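; BP_Counter1 is a counter Blueprint that shows a running count on a Text Render component.
; Each PressF event flips a Toggle flag and increments Count only when the flag becomes true, so the displayed number rises on every other press.
; Unconnected graph fragments hold a decrement and a wrap-to-zero count up to nine, and the Play and Stop function is an empty stub.
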(event `/Game/FirstGame/BP_0828/BPI_Switch.Press F`
  (bind _output_get (set `self.Toggle` (not (`self.Toggle`))))
  (if _output_get
    ; Count를 1증가
    (set `self.Count` (+ (`self.Count`) 1))
    ; Count값을 Text Render에 표시
    (`TextRenderComponent.K2_SetText` (`self.TextRender`) (`KismetTextLibrary.Conv_IntToText` (`self.Count`) false true 1 244))))

(fn `Play and Stop`
  (params (`Is Play` :type Boolean))
  (returns (bResult :type Boolean)))

(fn `UserConstructionScript`)