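; BP_MOVERect6 is a Blueprint that moves its StaticMesh in an endless plus-shaped path around the relative origin in the X-Z plane.
; Tick switches on the 실린더 enum, an eight-state machine that goes out and back along +Z, +X, -Z, then -X.
; Each state adds a fixed relative step per frame without sweep, so speed depends on frame rate, and advances when the mesh reaches its limit.
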(event `self.ReceiveTick`
  (params (DeltaSeconds :type "Float (single-precision)"))
  (bind _relativelocation_x (`KismetMathLibrary.BreakVector` (`SceneComponent.RelativeLocation` (`self.StaticMesh`))))
  (bind _relativelocation_x_2 (`KismetMathLibrary.BreakVector` (`SceneComponent.RelativeLocation` (`self.StaticMesh`))))
  (bind (_relativelocation_x_3 _relativelocation_y _relativelocation_z) (`KismetMathLibrary.BreakVector` (`SceneComponent.RelativeLocation` (`self.StaticMesh`))))
  (bind (_relativelocation_x_4 _relativelocation_y_2 _relativelocation_z_2) (`KismetMathLibrary.BreakVector` (`SceneComponent.RelativeLocation` (`self.StaticMesh`))))
  (bind _relativelocation_x_5 (`KismetMathLibrary.BreakVector` (`SceneComponent.RelativeLocation` (`self.StaticMesh`))))
  (bind (_relativelocation_x_6 _relativelocation_y_3 _relativelocation_z_3) (`KismetMathLibrary.BreakVector` (`SceneComponent.RelativeLocation` (`self.StaticMesh`))))
  (bind _relativelocation_x_7 (`KismetMathLibrary.BreakVector` (`SceneComponent.RelativeLocation` (`self.StaticMesh`))))
  (bind (_relativelocation_x_8 _relativelocation_y_4 _relativelocation_z_4) (`KismetMathLibrary.BreakVector` (`SceneComponent.RelativeLocation` (`self.StaticMesh`))))
  (switch `/Game/FirstGame/ENUM_MovType6` (`self.실린더`)
    (:`NewEnumerator0`
      ; 위로 움직인다.
      (set `self.실린더` "NewEnumerator0")
      (`SceneComponent.K2_AddRelativeLocation` (`self.StaticMesh`) (0.0 0.0 10.0) false false)
      (if (>= _relativelocation_z_3 500.0)
        (set `self.실린더` "NewEnumerator1")))
    (:`NewEnumerator1`
      (set `self.실린더` "NewEnumerator1")
      (`SceneComponent.K2_AddRelativeLocation` (`self.StaticMesh`) (0.0 0.0 -10.0) false false)
      (if (<= _relativelocation_z_4 0.0)
        (set `self.실린더` "NewEnumerator2")))
    (:`NewEnumerator2`
      (set `self.실린더` "NewEnumerator2")
      (`SceneComponent.K2_AddRelativeLocation` (`self.StaticMesh`) (10.0 0.0 0.0) false false)
      (if (>= _relativelocation_x 500.0)
        (set `self.실린더` "NewEnumerator3")))
    (:`NewEnumerator3`
      (set `self.실린더` "NewEnumerator3")
      (`SceneComponent.K2_AddRelativeLocation` (`self.StaticMesh`) (-10.0 0.0 0.0) false false)
      (if (<= _relativelocation_x_2 0.0)
        (set `self.실린더` "NewEnumerator4")))
    (:`NewEnumerator4`
      (set `self.실린더` "NewEnumerator4")
      (`SceneComponent.K2_AddRelativeLocation` (`self.StaticMesh`) (0.0 0.0 -10.0) false false)
      (if (<= _relativelocation_z -500.0)
        (set `self.실린더` "NewEnumerator5")))
    (:`NewEnumerator5`
      (set `self.실린더` "NewEnumerator5")
      (`SceneComponent.K2_AddRelativeLocation` (`self.StaticMesh`) (0.0 0.0 10.0) false false)
      (if (>= _relativelocation_z_2 0.0)
        (set `self.실린더` "NewEnumerator6")))
    (:`NewEnumerator6`
      (set `self.실린더` "NewEnumerator6")
      (`SceneComponent.K2_AddRelativeLocation` (`self.StaticMesh`) (-10.0 0.0 0.0) false false)
      (if (<= _relativelocation_x_5 -500.0)
        (set `self.실린더` "NewEnumerator7")))
    (:`NewEnumerator7`
      (set `self.실린더` "NewEnumerator7")
      (`SceneComponent.K2_AddRelativeLocation` (`self.StaticMesh`) (10.0 0.0 0.0) false false)
      (if (>= _relativelocation_x_7 0.0)
        (set `self.실린더` "NewEnumerator0")))))

(fn `UserConstructionScript`)