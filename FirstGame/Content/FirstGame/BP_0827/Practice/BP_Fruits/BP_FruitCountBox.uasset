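; BP_FruitCountBox is a practice counter that displays a running fruit count on a TextRender component.
; The DoGet event adds one to Count and DoGet1 subtracts one, each then refreshing the text through ShowCount, which also runs on BeginPlay.
; It has no overlap logic of its own, although its comments tie the count changes to fruit overlaps.
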(event `self.ReceiveBeginPlay`
  (`self.Show Count`))

(event `/Game/FirstGame/BP_0827/Practice/BP_Fruits/BPI_Fruits.Do Get`
  (`self.Count Add one `))

(event `/Game/FirstGame/BP_0827/Practice/BP_Fruits/BPI_Fruits.Do Get1`
  (`self.Count Subtract One`))

(fn `Count Add one `
  ; Fruit에 overlap되면 Count가 1씩 증가한다.
  (set `self.Count` (+ (`self.Count`) 1))
  (`self.Show Count`))

(fn `Count Subtract One`
  ; Fruit에 overlap되면 Count가 1씩 감소한다.
  (set `self.Count` (- (`self.Count`) 1))
  (`self.Show Count`))

(fn `Show Count`
  (`TextRenderComponent.K2_SetText` (`self.TextRender`) (`KismetTextLibrary.Conv_IntToText` (`self.Count`))))

(fn `UserConstructionScript`)